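; Sky sphere Blueprint that drives time-of-day lighting, cloud cover and rain, from an initial time or the game manager's clock.
; RefreshSky pitches the directional light by time, then RefreshCloudy dims it and updates the dynamic sky material using sun-height color curves or manual colors.
; Skylight recapture is throttled to a game-minute interval to protect frame rate, unless forced or the day wraps.
; RefreshRain toggles and scales the rain particle system.
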(fn ConstructionScript
  (bind _inittime (Variables|SkyParam|GetInitTime))
  (bind (_x _y _z) (Utilities|Struct|BreakIntVector _inittime))
  (bind _returnvalue (Rendering|Material|CreateDynamicMaterialInstance (Variables|BP_Skydome|GetSky%20Sphere%20mesh) 0 "/Engine/EngineSky/M_Sky_Panning_Clouds2.M_Sky_Panning_Clouds2" "None" :!class /Script/Engine.PrimitiveComponent))
  (Variables|Default|SetSky%20material _returnvalue)
  (if (Variables|Default|GetRefresh%20material) ; Updating bool in details panel causes construction script to run again
    _
    (else
      _))
  (Variables|Default|SetRefresh%20material false)
  (CallFunction|RefreshSky _x _y _z true)
  (CallFunction|RefreshRain (Variables|SkyParam|GetrainFallValue)))

(fn UpdateSunDirection
  (bind _sky_material (Variables|Default|GetSky%20material))
  (bind _sky_material_2 (Variables|Default|GetSky%20material))
  (Rendering|Material|SetVectorParameterValue _sky_material "Light direction" (Math|Conversions|ToLinearColor(Vector) (Math|Rotator|GetRotationXVector (Variables|/Script/Engine.SceneComponent|GetRelativeRotation (Variables|Default|GetDirectionalLight)))) :!class /Script/Engine.MaterialInstanceDynamic)
  (Rendering|Material|SetVectorParameterValue _sky_material "Sun color" (Math|Conversions|ToLinearColor(Color) (Variables|/Script/Engine.LightComponentBase|GetLightColor (Variables|Default|GetDirectionalLight))) :!class /Script/Engine.MaterialInstanceDynamic)
  (Variables|Overridesettings|SetSun%20height (Math|Float|MapRangeUnclamped (.Pitch (Math|Rotator|BreakRotator (Variables|/Script/Engine.SceneComponent|GetRelativeRotation (Variables|Default|GetDirectionalLight)))) 0.0 -9e+01 0.0 1.0))
  (Rendering|Material|SetVectorParameterValue _sky_material_2 "Horizon color" (Class|CurveLinearColor|GetClampedLinearColorValue (Variables|Default|GetHorizon%20color%20curve) (Variables|Overridesettings|GetSun%20height)) :!class /Script/Engine.MaterialInstanceDynamic)
  (Rendering|Material|SetVectorParameterValue _sky_material_2 "Zenith color" (Class|CurveLinearColor|GetClampedLinearColorValue (Variables|Default|GetZenith%20color%20curve) (Variables|Overridesettings|GetSun%20height)) :!class /Script/Engine.MaterialInstanceDynamic)
  (Rendering|Material|SetVectorParameterValue _sky_material_2 "Cloud color" (Class|CurveLinearColor|GetClampedLinearColorValue (Variables|Default|GetCloud%20color%20curve) (Variables|Overridesettings|GetSun%20height)) :!class /Script/Engine.MaterialInstanceDynamic)
  (Rendering|Material|SetScalarParameterValue _sky_material_2 "Horizon falloff" (Math|Float|Lerp 3.0 8.0 (Math|Float|Absolute(Float) (Variables|Overridesettings|GetSun%20height))) :!class /Script/Engine.MaterialInstanceDynamic)
  (Rendering|Material|SetScalarParameterValue _sky_material_2 "Sun height" (Math|Float|SelectFloat (Math|Float|Absolute(Float) (Variables|Overridesettings|GetSun%20height)) 0.0 (< (Variables|Overridesettings|GetSun%20height) 0.0)) :!class /Script/Engine.MaterialInstanceDynamic))

(fn RefreshMaterial
  (bind _sky_material (Variables|Default|GetSky%20material))
  (bind _sky_material_2 (Variables|Default|GetSky%20material))
  (bind _sky_material_3 (Variables|Default|GetSky%20material))
  (bind _sky_material_4 (Variables|Default|GetSky%20material))
  (bind _sky_material_5 (Variables|Default|GetSky%20material))
  (Utilities|IsValid (Variables|Default|GetDirectionalLight) ; Has a directional light been assigned?
    (:Is%20Valid
      (Rendering|Material|SetVectorParameterValue _sky_material_3 "Light direction" (Math|Conversions|ToLinearColor(Vector) (Math|Rotator|GetRotationXVector (Variables|/Script/Engine.SceneComponent|GetRelativeRotation (Variables|Default|GetDirectionalLight)))) :!class /Script/Engine.MaterialInstanceDynamic)
      (Rendering|Material|SetVectorParameterValue _sky_material_3 "Sun color" (Math|Conversions|ToLinearColor(Color) (Variables|/Script/Engine.LightComponentBase|GetLightColor (Variables|Default|GetDirectionalLight))) :!class /Script/Engine.MaterialInstanceDynamic)
      (Variables|Overridesettings|SetSun%20height (Math|Float|MapRangeUnclamped (.Pitch (Math|Rotator|BreakRotator (Variables|/Script/Engine.SceneComponent|GetRelativeRotation (Variables|Default|GetDirectionalLight)))) 0.0 -9e+01 0.0 1.0)))
    (:Is%20Not%20Valid
      (Rendering|Material|SetVectorParameterValue _sky_material_2 "Light direction" (Math|Conversions|ToLinearColor(Vector) (Math|Rotator|GetRotationXVector (Math|Rotator|MakeRotator 0.0 (Math|Float|MapRangeUnclamped (Variables|Overridesettings|GetSun%20height) -1.0 1.0 9e+01 -9e+01) (.Yaw (Math|Rotator|BreakRotator (Transformation|GetActorRotation)))))) :!class /Script/Engine.MaterialInstanceDynamic)
      (Rendering|Material|SetVectorParameterValue _sky_material_2 "Sun color" (Math|Color|Lerp(LinearColor) "(R=1.000000,G=0.221000,B=0.040000,A=1.000000)" "(R=0.954000,G=0.901000,B=0.744120,A=1.000000)" (Math|Float|Clamp(Float) (+ (Variables|Overridesettings|GetSun%20height) 0.2))) :!class /Script/Engine.MaterialInstanceDynamic)))
  (if (Variables|Default|GetColors%20determined%20by%20sun%20position)
    (Rendering|Material|SetVectorParameterValue _sky_material_4 "Horizon color" (Class|CurveLinearColor|GetClampedLinearColorValue (Variables|Default|GetHorizon%20color%20curve) (Variables|Overridesettings|GetSun%20height)) :!class /Script/Engine.MaterialInstanceDynamic)
    (Rendering|Material|SetVectorParameterValue _sky_material_4 "Zenith color" (Class|CurveLinearColor|GetClampedLinearColorValue (Variables|Default|GetZenith%20color%20curve) (Variables|Overridesettings|GetSun%20height)) :!class /Script/Engine.MaterialInstanceDynamic)
    (Rendering|Material|SetVectorParameterValue _sky_material_4 "Cloud color" (- (Class|CurveLinearColor|GetClampedLinearColorValue (Variables|Default|GetCloud%20color%20curve) (Variables|Overridesettings|GetSun%20height)) (* (* "(R=1.000000,G=1.000000,B=1.000000,A=1.000000)" (Variables|SkyParam|GetcloudyValue)) 0.7)) :!class /Script/Engine.MaterialInstanceDynamic)
    (Rendering|Material|SetScalarParameterValue _sky_material_4 "Horizon falloff" (Math|Float|Lerp 3.0 7.0 (Math|Float|Absolute(Float) (Variables|Overridesettings|GetSun%20height))) :!class /Script/Engine.MaterialInstanceDynamic)
    (else
      (Rendering|Material|SetVectorParameterValue _sky_material "Horizon color" (Variables|Overridesettings|GetHorizon%20color) :!class /Script/Engine.MaterialInstanceDynamic)
      (Rendering|Material|SetVectorParameterValue _sky_material "Zenith color" (Variables|Overridesettings|GetZenith%20Color) :!class /Script/Engine.MaterialInstanceDynamic)
      (Rendering|Material|SetVectorParameterValue _sky_material "Overall color" (Variables|Overridesettings|GetOverall%20Color) :!class /Script/Engine.MaterialInstanceDynamic)
      (Rendering|Material|SetVectorParameterValue _sky_material "Cloud color" (Variables|Overridesettings|GetCloud%20color) :!class /Script/Engine.MaterialInstanceDynamic)
      (Rendering|Material|SetScalarParameterValue _sky_material "Horizon falloff" (Variables|Overridesettings|GetHorizon%20Falloff) :!class /Script/Engine.MaterialInstanceDynamic)))
  (Rendering|Material|SetScalarParameterValue _sky_material_5 "Cloud speed" (Variables|Default|GetCloud%20speed) :!class /Script/Engine.MaterialInstanceDynamic)
  (Rendering|Material|SetScalarParameterValue _sky_material_5 "Sun brightness" (Variables|Default|GetSun%20brightness) :!class /Script/Engine.MaterialInstanceDynamic)
  (Rendering|Material|SetScalarParameterValue _sky_material_5 "Sun height" (Math|Float|SelectFloat (Math|Float|Absolute(Float) (Variables|Overridesettings|GetSun%20height)) 0.0 (< (Variables|Overridesettings|GetSun%20height) 0.0)) :!class /Script/Engine.MaterialInstanceDynamic)
  (Rendering|Material|SetScalarParameterValue _sky_material_5 "Cloud opacity" (Variables|Default|GetCloud%20opacity) :!class /Script/Engine.MaterialInstanceDynamic)
  (Rendering|Material|SetScalarParameterValue _sky_material_5 "Stars brightness" (Variables|Default|GetStars%20brightness) :!class /Script/Engine.MaterialInstanceDynamic))

(fn RefreshSky
  (params (hour :type Integer) (minute :type Integer) (second :type Integer) (force :type Boolean))
  ;[1 1 1] 将当前时间兑换成分钟
  (LocalVariables|SetallMinutes (+ (* hour 60) minute))
  (Utilities|FlowControl|Sequence
    (:then_0
      ;[1 1 1] 刷新天空和光照
      (Transformation|SetRelativeRotation (Variables|Default|GetDirectionalLight) (Math|Rotator|MakeRotator 0.0 (- 0.0 (/ (- (+ (/ (Math|Conversions|ToFloat(Integer) second) 6e+01) (Math|Conversions|ToFloat(Integer) (LocalVariables|GetallMinutes))) 3.6e+02) 4.0)) 0.0) false false)
      (CallFunction|RefreshCloudy (Variables|SkyParam|GetcloudyValue)))
    (:then_1
      ;[1 1 1] 跨天判断，如果传入时间少于当前时间，认为是跨天，强制刷新
      (LocalVariables|SetisForce (or force (> (Variables|Default|GetcurrentMinute) (LocalVariables|GetallMinutes))))
      ;[1 1 1] 判断间隔时间
      (if (or (!= (LocalVariables|GetallMinutes) (Variables|Default|GetcurrentMinute)) (LocalVariables|GetisForce))
        (bind _output_get (Variables|Default|SetcurrentMinute (LocalVariables|GetallMinutes)))
        (if (or (> _output_get (+ (Variables|Default|GetlastRefreshMinute) (Variables|Default|GetminuteIntervalEveryRefresh))) (LocalVariables|GetisForce))
          (Variables|Default|SetlastRefreshMinute _output_get)
          ;[1 1 1] 刷新环境光，频繁刷新会导致帧率下降
          (Class|SkyLightComponent|RecaptureSky (Variables|Default|GetSkyLight)))))))

(fn RefreshRain
  (params (rainFallValue :type Integer))
  (bind _rainparticlesystem (Variables|Default|GetRainParticleSystem))
  (bind _output_get (Variables|SkyParam|SetrainFallValue rainFallValue))
  (if (> _output_get 0)
    (Components|Activation|SetActive _rainparticlesystem true false)
    (Effects|Components|ParticleSystem|SetFloatParameter _rainparticlesystem "RainFallMax" (Math|Conversions|ToFloat(Integer) (Variables|SkyParam|GetrainFallValue)))
    (Effects|Components|ParticleSystem|SetFloatParameter _rainparticlesystem "RainFallRipMax" (Math|Conversions|ToFloat(Integer) (/ (Variables|SkyParam|GetrainFallValue) 20)))
    (else
      (Components|Activation|SetActive _rainparticlesystem false false))))

(fn RefreshCloudy
  (params (cloudyValue :type Float%20%28single-precision%29))
  (bind _output_get (Variables|SkyParam|SetcloudyValue cloudyValue))
  (Variables|Default|SetCloud%20opacity (* _output_get 3.0))
  (Rendering|Components|Light|SetIntensity (Variables|Default|GetDirectionalLight) (- 1e+01 (* _output_get 7.0)))
  (CallFunction|RefreshMaterial))

(fn RefreshSkybyGameTime
  (bind _returnvalue (Class|CommonBlueprintFunctionLibrary|GetMainGameManager))
  (bind _returnvalue_2 (Class|MainGameManager|GetUserData _returnvalue))
  (bind _returnvalue_3 (Class|UserData|GetGameTimeData _returnvalue_2))
  (bind _returnvalue_4 (Class|CommonBlueprintFunctionLibrary|GetHours _returnvalue_3))
  (bind _returnvalue_5 (Class|CommonBlueprintFunctionLibrary|GetMinutes _returnvalue_3))
  (bind _returnvalue_6 (Class|CommonBlueprintFunctionLibrary|GetSeconds _returnvalue_3))
  (CallFunction|RefreshSky _returnvalue_4 _returnvalue_5 _returnvalue_6 false))