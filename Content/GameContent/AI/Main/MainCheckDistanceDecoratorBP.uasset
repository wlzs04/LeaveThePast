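; Behavior tree decorator that gates an AI branch on the controlled pawn being at least a set Distance away from a target actor.
; It reads the actor from the DataKey blackboard key and compares the straight-line 3D distance between the two locations against Distance.
; The check fails when either the pawn or the blackboard actor is invalid.
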(fn PerformConditionCheckAI
  (params (OwnerController :type AI%20Controller%20Object%20Reference) (ControlledPawn :type Pawn%20Object%20Reference))
  (bind _datakey (Variables|Default|GetdataKey))
  (bind _returnvalue (AI|BehaviorTree|GetBlackboardValueasActor _datakey))
  (Utilities|IsValid ControlledPawn
    (:Is%20Valid
      (Utilities|IsValid _returnvalue
        (:Is%20Valid
          (return (>= (Math|Vector|VectorLength (- (Transformation|GetActorLocation ControlledPawn) (Transformation|GetActorLocation _returnvalue))) (Variables|Default|Getdistance))))
        (:Is%20Not%20Valid
          _)))
    (:Is%20Not%20Valid
      _))
  (return false))