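; Main player controller Blueprint that toggles the system menu when the System input action is pressed.
; An InSystem flag picks the branch and flips afterward, with the MainGameModeBP cast from the game mode showing or hiding the menu UI.
; Opening the menu disables input on player pawn 0 and shows the mouse cursor, while closing it reverses both.
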(event EventBeginPlay)

(event EventTick
  (params (DeltaSeconds :type Float%20%28single-precision%29)))

(event Input|ActionEvents|InputActionSystem
  (params (Key :type Key%20Structure))
  (bind _returnvalue (Game|Player|GetPlayerPawn 0))
  (:Pressed
    (if (Variables|Default|GetinSystem)
      (bind _asmain_game_mode_bp (Utilities|Casting|CastToMainGameModeBP (Game|GetGameMode)))
      (Default|HideMenuUI _asmain_game_mode_bp)
      (Input|EnableInput _returnvalue 0)
      (Variables|Default|SetbShowMouseCursor false)
      (else
        (bind _asmain_game_mode_bp_2 (Utilities|Casting|CastToMainGameModeBP (Game|GetGameMode)))
        (Default|ShowMenuUI _asmain_game_mode_bp_2)
        (Input|DisableInput _returnvalue 0)
        (Variables|Default|SetbShowMouseCursor true)))
    (Variables|Default|SetinSystem (not (Variables|Default|GetinSystem)))))

(fn ConstructionScript)