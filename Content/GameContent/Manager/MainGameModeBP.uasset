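; MainGameModeBP is the game mode, offering helper functions for showing message tips.
; On BeginPlay it casts the game instance to MainGameManager and caches it.
; ShowMessageTip prints a given value directly.
; ShowMessageTipById uses the manager's config manager to look up the tip text by ID in the MessageTipRecorder config, then displays it with PrintString.
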(event EventBeginPlay
  (bind _asmain_game_manager (Utilities|Casting|CastToMainGameManager (Game|GetGameInstance)))
  (Variables|Default|SetgameManager _asmain_game_manager))

(event EventTick
  (params (DeltaSeconds :type Float%20%28single-precision%29)))

(fn ConstructionScript)

(fn ShowMessageTip
  (params (value :type String))
  (Development|PrintString value))

(fn ShowMessageTipbyId
  (params (id :type Integer))
  (bind _returnvalue (Class|MainGameManager|GetConfigManager (Variables|Default|GetgameManager)))
  (bind _returnvalue_2 (Class|ConfigManager|GetConfigbyName _returnvalue "/Script/LeaveThePast.MessageTipRecorder"))
  (bind _returnvalue_3 (Class|RecorderBase|GetValuebyName (.Value (Utilities|Map|Find _returnvalue_2 id)) "value"))
  (Development|PrintString _returnvalue_3))